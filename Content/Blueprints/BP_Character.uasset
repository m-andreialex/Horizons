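; BP_Character is a character Blueprint that creates the W_HUD widget and delegates parkour and fall-damage logic to its components.
; BeginPlay gives ParkourComp a self reference and the default gravity scale.
; Tick drives the component's WRUpdate through a short Delay, throttling it to roughly fixed intervals.
; On landing, it applies Health's velocity-based fall damage to itself and notifies ParkourComp.
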(event EventBeginPlay
  (bind _parkourcomp (Variables|Default|GetParkourComp))
  (bind _returnvalue (UserInterface|CreateWidget "/Game/Resources/Widgets/W_HUD.W_HUD_C" (Game|GetPlayerController 0)))
  (UserInterface|Viewport|AddtoViewport _returnvalue 0)
  (Variables|/Script/Horizons.ParkourComponent|SetCharacter _parkourcomp self)
  (Class|ParkourComponent|SetDefaultGrav _parkourcomp (Variables|/Script/Engine.CharacterMovementComponent|GetGravityScale (Variables|Character|GetCharacterMovement))))

(event EventTick
  (params (DeltaSeconds :type Float%20%28single-precision%29))
  (Utilities|FlowControl|Delay 0.02)
  (Class|ParkourComponent|WRUpdate (Variables|Default|GetParkourComp)))

(event EventOnLanded
  (params (Hit :type Hit%20Result%20Structure%20%28by%20ref%29))
  (bind _self self)
  (Game|Damage|ApplyDamage _self (Class|HealthComponent|CalcFallDamage (Variables|Default|GetHealth) (Math|Vector|VectorLength (Transformation|GetVelocity)) 1000 0.1) 0 _self "/Script/Engine.DamageType")
  (Class|ParkourComponent|OnLanding (Variables|Default|GetParkourComp)))

(fn ConstructionScript)